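; Walls actor for MazePlanet that positions its forward and back walls at configurable depths when play begins.
; BeginPlay sets ForwardWall and BackWallBasePoint relative X locations from the depth variables by teleporting, then prints the actor transform as long-lived debug text.
; The Hit event only casts the other actor to Player and takes no further action.
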(event EventBeginPlay
  (CallFunction|ChangeForwardWallDepth)
  (CallFunction|ChangeBackWallDepth)
  (Development|PrintString (Utilities|String|Append "WallTransform" (Utilities|String|ToString(Transform) (Transformation|GetActorTransform))) true true "(R=0.000000,G=0.435000,B=0.011465,A=1.000000)" 6e+01))

(event Collision|EventActorBeginOverlap
  (params (OtherActor :type Actor%20Object%20Reference)))

(event EventTick
  (params (DeltaSeconds :type Float%20%28single-precision%29)))

(event Collision|EventHit
  (params (MyComp :type Primitive%20Component%20Object%20Reference) (Other :type Actor%20Object%20Reference) (OtherComp :type Primitive%20Component%20Object%20Reference) (bSelfMoved :type Boolean) (HitLocation :type Vector :default "0, 0, 0") (HitNormal :type Vector :default "0, 0, 0") (NormalImpulse :type Vector :default "0, 0, 0") (Hit :type Hit%20Result%20Structure%20%28by%20ref%29))
  (Utilities|Casting|CastToPlayer Other))

(fn ConstructionScript)

(fn ChangeForwardWallDepth
  (Transformation|SetRelativeLocation (Variables|Default|GetForwardWall) (Math|Vector|MakeVector (Variables|Default|GetForwardWallDepth) 0.0 0.0) false true))

(fn ChangeBackWallDepth
  (Transformation|SetRelativeLocation (Variables|Default|GetBackWallBasePoint) (Math|Vector|MakeVector (Variables|Default|GetBackWallDepth) 0.0 0.0) false true))