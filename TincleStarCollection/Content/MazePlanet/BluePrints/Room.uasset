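; Room actor for MazePlanet that builds its ceiling and floor from spawned CeilingAndFloor tile actors.
; ChangeWallPosition runs a nested X/Y loop, with bounds taken from the remainder (%) of the wall depth spans by tile scale.
; Each tile spawns at a grid offset, joins CeilingAndFloorArray, then attaches to RoomOffset with SnapToTarget location, which overrides that offset.
; The events and construction script are empty, and nothing here calls the function.
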(event EventBeginPlay)

(event Collision|EventActorBeginOverlap
  (params (OtherActor :type Actor%20Object%20Reference)))

(event EventTick
  (params (DeltaSeconds :type Float%20%28single-precision%29)))

(fn ConstructionScript)

(fn ChangeWallPosition
  (params (oneTileScale :type Float%20%28single-precision%29))
  (for _index (range 0 (Math|Float|Truncate (Math|Float|%(Float) (- (Variables|Default|GetForwardWallDepth) (Variables|Default|GetBackWallDepth)) oneTileScale)))
    (for _index_2 (range 0 (Math|Float|Truncate (Math|Float|%(Float) (- (Variables|Default|GetRightWallDepth) (Variables|Default|GetLeftWallDepth)) oneTileScale)))
      (bind _returnvalue (Game|SpawnActorfromClass "/Game/MazePlanet/BluePrints/CeilingAndFloor.CeilingAndFloor_C" (Math|Transform|MakeTransform (Math|Vector|MakeVector (* _index oneTileScale) (* _index_2 oneTileScale) 0.0)) "Undefined" 0 0))
      (Utilities|Array|Add (Variables|Default|GetCeilingAndFloorArray) _returnvalue)
      (Transformation|AttachComponentToComponent _returnvalue (Variables|Default|GetRoomOffset) "None" "SnapToTarget" "SnapToTarget" "KeepRelative" true))))