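; StarSpawner keeps waves of collectible TwincleStar actors appearing around the planet in the MazePlanet main game scene.
; On BeginPlay it pre-spawns an inactive pool, wiring each star to the planet, explorer and score manager and adding it to the player's look-ignore list.
; During one TimeManager game state, Tick respawns the pool as a new wave once every star is inactive.
; ClearStars deactivates the whole pool.
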(event Custom|ClearStars
  (for _array_element (Variables|Default|GetStarList)
    (Default|Deactive _array_element)))

(event EventBeginPlay
  (|CreateStar (Variables|Default|GetOneWaveStarNum)))

(event EventTick
  (params (DeltaSeconds :type Float%20%28single-precision%29))
  (if (Utilities|Enum|Equal(Enum) "NewEnumerator1" (Variables|/Game/MazePlanet/BluePrints/MainGameScene/TimeManager.TimeManager_C|GetCurGameState (Variables|Default|GetTimeManager)))
    (|CheckAndSpawnStars)))

(fn ConstructionScript)

(fn CheckAllStarDeactive
  (for _array_element (Variables|Default|GetStarList)
    (bind _isactive (Default|GetIsActive _array_element))
    (if _isactive
      (return false)))
  (return true))

(fn SpawnStar
  (params (SpawnNum :type Integer) (spawnDistanceRate :type Float%20%28single-precision%29))
  (bind (_array_element _array_index) (Utilities|Array|ForEachLoopwithBreak (Variables|Default|GetStarList) :!label _label)
    (:LoopBody
      (Default|Spawn _array_element (* _array_index spawnDistanceRate) true)
      (if (>= _array_index SpawnNum)
        (goto _label Break)))))