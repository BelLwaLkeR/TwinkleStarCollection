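; Audio manager for the MazePlanet main game scene that controls background music pitch and crossfades between tracks.
; Tick steps Pitch toward TargetPitch along a precomputed direction, clamping on overshoot and applying it to the current BGM.
; Tick also starts any assigned NextBGM silent, then ramps complementary volumes by a fixed per-frame step.
; ChangeGenerationBGM, which would stop the old track and promote the next, is never reached.
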(event Custom|ChangeMusic
  (params (NextBGM :type Ambient%20Sound%20Object%20Reference))
  (if (== (Variables|Default|GetNextBGM) 0)
    (Variables|Default|SetNextBGM NextBGM)))

(event Custom|ChangePitch
  (params (NewPitch :type Float%20%28single-precision%29))
  (Variables|Default|SettargetPitch NewPitch)
  (|SetTargetVector))

(event EventBeginPlay
  (Audio|Components|Audio|SetPitchMultiplier (Variables|/Script/Engine.AmbientSound|GetAudioComponent (Variables|Default|GetBGM)) (Variables|Default|GetPitch)))

(event Collision|EventActorBeginOverlap
  (params (OtherActor :type Actor%20Object%20Reference)))

(event EventTick
  (params (DeltaSeconds :type Float%20%28single-precision%29))
  (|ChangePitchProcess)
  (|CrossFadeProcess))

(fn ConstructionScript)