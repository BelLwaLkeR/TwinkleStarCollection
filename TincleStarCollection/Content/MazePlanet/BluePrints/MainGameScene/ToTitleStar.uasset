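; ToTitleStar is a collectible star that returns the game to the Title level when the explorer touches it.
; It spawns offset from the player camera, then spins and falls toward the planet until a distance check snaps it into landed state.
; Each tick it follows the planet's height offset.
; Once landed, it rotates and tests squared distance to the explorer, playing a sound and loading Title after a short delay.
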(event Custom|Spawn
  (|SpawnStar))

(event Custom|GetStar
  (Variables|Default|SetisActive false)
  (Audio|PlaySound2D "/Game/MazePlanet/Sounds/get2.get2")
  (Utilities|FlowControl|Delay 1.0)
  (Game|OpenLevel(byName) "Title"))

(event EventBeginPlay
  (CallFunction|Spawn)
  (Variables|Default|SetisActive true))

(event EventTick
  (params (DeltaSeconds :type Float%20%28single-precision%29))
  (|SetHeightOffsetFromPlanet)
  (if (Variables|Default|GetisLanding)
    (CallFunction|Landing 0.5)
    (if (Variables|Default|GetisActive)
      (|CheckHitExplorer))
    (else
      (CallFunction|Falling 6.0 1.0))))

(fn ConstructionScript)

(fn Landing
  (params (RotationSpeed :type Float%20%28single-precision%29))
  (Transformation|AddLocalRotation (Variables|Default|GetStaticMesh) (Math|Vector|RotatorfromAxisandAngle (Math|Vector|Normalize (- (Transformation|GetWorldLocation (Variables|/Game/MazePlanet/BluePrints/Planet.Planet_C|GetSphere (Variables|Default|GetPlanetActor))) (Transformation|GetWorldLocation (Variables|Default|GetStaticMesh)))) RotationSpeed) false false))

(fn Falling
  (params (RollingSpeedDegree :type Float%20%28single-precision%29) (FallSpeed :type Float%20%28single-precision%29))
  (Transformation|AddLocalRotation (Variables|Default|GetStaticMesh) (Math|Rotator|MakeRotator 0.0 0.0 RollingSpeedDegree) false false)
  (Transformation|AddActorWorldOffset (|fallingOffset FallSpeed) false true)
  (if (|isLandingBorder)
    (Transformation|SetActorLocation (|calcNewPosition) false true)
    (Variables|Default|SetisLanding true)))

(fn RandomFloat
  (params (min :type Float%20%28single-precision%29) (max :type Float%20%28single-precision%29))
  (return (+ min (* (Math|Random|RandomFloat) (- max min)))))

(fn GetIsActive
  (return (Variables|Default|GetisActive)))