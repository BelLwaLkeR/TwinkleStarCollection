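; WalkSignBoardInGame is a signboard actor in the MazePlanet main game scene that points toward a target star, ToGameStar.
; It hides its left and right text renders at BeginPlay.
; Each Tick, while that star is valid and active, it shows the text and sets its yaw to the look-at direction from the Planet to the star, keeping pitch and roll.
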(event EventBeginPlay
  (Rendering|SetVisibility (Variables|Default|GetTextRenderR) false false))

(event Collision|EventActorBeginOverlap
  (params (OtherActor :type Actor%20Object%20Reference)))

(event EventTick
  (params (DeltaSeconds :type Float%20%28single-precision%29))
  (bind _returnvalue (Transformation|GetActorRotation))
  (bind _togamestar (Variables|Default|GettoGameStar))
  (bind (_roll _pitch) (Math|Rotator|BreakRotator _returnvalue))
  (if (!= _togamestar 0)
    (if (Variables|/Game/MazePlanet/BluePrints/MainGameScene/ToTitleStar.ToTitleStar_C|GetisActive _togamestar)
      (Transformation|SetActorRotation (Math|Rotator|MakeRotator _roll _pitch (.Yaw (Math|Rotator|BreakRotator (Math|Rotator|FindLookatRotation (Transformation|GetActorLocation (Variables|Default|Getplanet)) (Transformation|GetActorLocation (Variables|Default|GettoGameStar)))))) true)
      (Rendering|SetVisibility (Variables|Default|GetTextRenderR) true false))))

(fn ConstructionScript)