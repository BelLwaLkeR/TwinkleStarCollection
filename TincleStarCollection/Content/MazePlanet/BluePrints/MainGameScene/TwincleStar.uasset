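; Collectible star actor that falls toward a planet for the explorer to harvest for combo points.
; Spawn places it around the planet; it spins while falling, then rotates on the surface, following the planet's height offset each tick.
; A distance check or hit awards score, a popup and combo-pitched sound, while lifetime expiry resets the combo.
; Both outcomes hide and deactivate the actor instead of destroying it, so Spawn can reuse it.
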(event Custom|Burst
  (params (Combo :type Integer))
  (if (< Combo 8)
    (bind _pitch (CallFunction|GetPitch Combo))
    (Audio|PlaySound2D "/Game/MazePlanet/Sounds/get2.get2" 1.0 _pitch)
    (else
      (Audio|PlaySound2D "/Game/MazePlanet/Sounds/get1.get1" 1.0 1.0)))
  (CallFunction|Deactive))

(event Custom|Spawn
  (params (OffsetDistanceToPlanet :type Float%20%28single-precision%29) (PlaySound :type Boolean))
  (|SpawnStar OffsetDistanceToPlanet 1.5e+02 PlaySound))

(event Custom|GetStar
  (bind (_point _score _combo) (Default|AddScore (Variables|Default|GetScoreManager)))
  (bind _returnvalue (Game|SpawnActorfromClass "/Game/MazePlanet/BluePrints/MainGameScene/PointPopup.PointPopup_C" (Transformation|GetWorldTransform (Variables|Default|GetStaticMesh)) "AlwaysSpawn" 0 1e+01 1.0))
  (Default|Setup _returnvalue (Transformation|GetWorldLocation (Variables|Default|GetStaticMesh)) (Transformation|GetWorldLocation (Variables|/Game/MazePlanet/BluePrints/Planet.Planet_C|GetSphere (Variables|Default|GetPlanetActor))) _point _combo)
  (CallFunction|Burst _combo))

(event Custom|SetExplorerActor
  (params (ExplorerActor :type BP%20Explorer%20Object%20Reference))
  (Variables|Default|SetExplorerActor ExplorerActor))

(event Custom|Lost
  (Audio|PlaySound2D "/Game/MazePlanet/Sounds/lost.lost" 1.0 0.8)
  (Default|ResetCombo (Variables|Default|GetScoreManager))
  (CallFunction|Deactive))

(event Custom|SetDeactive
  (Rendering|SetActorHiddenInGame true)
  (Variables|Default|SetisLanding false)
  (Variables|Default|SetisActive false))

(event Custom|SetActive
  (params (PlaySound :type Boolean))
  (Rendering|SetActorHiddenInGame false)
  (Variables|Default|SetisLanding false)
  (Variables|Default|SetisActive true)
  (if PlaySound
    (Audio|PlaySoundatLocation "/Game/MazePlanet/Sounds/manyfall.manyfall" (Transformation|GetActorLocation))))

(event Custom|Deactive
  (CallFunction|SetDeactive))

(event EventBeginPlay
  (CallFunction|Spawn 5e+05 false)
  (CallFunction|SetActive false))

(event EventTick
  (params (DeltaSeconds :type Float%20%28single-precision%29))
  (|SetHeightOffsetFromPlanet)
  (if (Variables|Default|GetisActive)
    (|CheckHitExplorer
      (:else
        (|CheckOverLifeSpan
          (:else
            (if (Variables|Default|GetisLanding)
              (CallFunction|Landing 0.5)
              (else
                (CallFunction|Falling 6.0 1.0)))))))))

(event Collision|EventHit
  (params (MyComp :type Primitive%20Component%20Object%20Reference) (Other :type Actor%20Object%20Reference) (OtherComp :type Primitive%20Component%20Object%20Reference) (bSelfMoved :type Boolean) (HitLocation :type Vector :default "0, 0, 0") (HitNormal :type Vector :default "0, 0, 0") (NormalImpulse :type Vector :default "0, 0, 0") (Hit :type Hit%20Result%20Structure%20%28by%20ref%29))
  (if (Variables|Default|GetisActive)
    (if (== Other (Variables|Default|GetExplorerActor))
      (CallFunction|GetStar)
      (elif (and (== Other (Variables|Default|GetPlanetActor)) (not (Variables|Default|GetisLanding)))
        (Variables|Default|SetisLanding true)))))

(fn ConstructionScript)

(fn Landing
  (params (RotationSpeed :type Float%20%28single-precision%29))
  (Transformation|AddLocalRotation (Variables|Default|GetStaticMesh) (Math|Vector|RotatorfromAxisandAngle (Math|Vector|Normalize (- (Transformation|GetWorldLocation (Variables|/Game/MazePlanet/BluePrints/Planet.Planet_C|GetSphere (Variables|Default|GetPlanetActor))) (Transformation|GetWorldLocation (Variables|Default|GetStaticMesh)))) RotationSpeed) false false))

(fn Falling
  (params (RollingSpeedDegree :type Float%20%28single-precision%29) (FallSpeed :type Float%20%28single-precision%29))
  (Transformation|AddLocalRotation (Variables|Default|GetStaticMesh) (Math|Rotator|MakeRotator 0.0 0.0 RollingSpeedDegree) false false)
  (Transformation|AddActorWorldOffset (* (Math|Vector|Normalize (- (Transformation|GetActorLocation (Variables|Default|GetPlanetActor)) (Transformation|GetActorLocation))) FallSpeed) false true)
  (if (|TooNearPlanet)
    (Transformation|SetActorLocation (|calcNewLocation) false true)
    (Variables|Default|SetisLanding true)))

(fn RandomFloat
  (params (min :type Float%20%28single-precision%29) (max :type Float%20%28single-precision%29))
  (return (+ min (* (Math|Random|RandomFloat) (- max min)))))

(fn GetIsActive
  (return (Variables|Default|GetisActive)))

(fn GetPitch
  (params (Index :type Integer))
  (return (Utilities|Array|Get(acopy) (Variables|Default|GetPitchList) (select (< Index (Utilities|Array|Length (Variables|Default|GetPitchList))) Index (Utilities|Array|LastIndex (Variables|Default|GetPitchList))))))