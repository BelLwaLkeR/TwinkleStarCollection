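; Round timer for the MazePlanet game scene that moves play through countdown, timed play and result states.
; Tick runs the current state's logic, comparing it with the previous state to detect entry.
; The timed phase updates the HMD clock, raises music pitch near the end, then switches music and spawns the return-to-title star.
; The result phase clears stars and draws the HMD result UI.
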(event Custom|BeginStartCountdown
  (Variables|Default|SetCouwntDownBeginTime (Math|DateTime|Now))
  (Variables|Default|SetCurGameState "NewEnumerator0"))

(event EventBeginPlay
  (Variables|Default|SetPreGameState "NewEnumerator1")
  (Variables|Default|SetCurGameState "NewEnumerator0"))

(event EventTick
  (params (DeltaSeconds :type Float%20%28single-precision%29))
  (switch Utilities|FlowControl|Switch|SwitchonInGameState (Variables|Default|GetCurGameState)
    (:NewEnumerator0
      (|CountDown))
    (:NewEnumerator1
      (|InGameTimeCount 59))
    (:NewEnumerator2
      (|Resoult))))

(fn ConstructionScript)