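; PointPopup is a score popup actor that shows earned points and any combo count as floating text around a planet.
; Setup places and reveals the initially hidden text, facing it away from the planet's location, with pitch flattened unless it pops below that location.
; Each tick moves the text along its own up vector at a set speed, then destroys the actor once its lifetime since Setup has elapsed.
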(event Custom|Setup
  (params (locaiton :type Vector) (planetLocation :type Vector) (point :type Integer) (combo :type Integer))
  (Transformation|SetWorldLocationAndRotation (Variables|Default|Gettext) locaiton (|MakeRotation locaiton planetLocation) false true)
  (Rendering|Components|TextRender|SetText (Variables|Default|Gettext) (|MakeText point combo))
  (Development|SetHiddeninGame (Variables|Default|Gettext) false false)
  (Variables|Default|SetspawinTimeSec (Math|DateTime|Now)))

(event EventBeginPlay
  (Development|SetHiddeninGame (Variables|Default|Gettext) true false))

(event EventTick
  (params (DeltaSeconds :type Float%20%28single-precision%29))
  (|DestroyIfTimeOver
    (:false
      (Transformation|SetWorldLocation (Variables|Default|Gettext) (|MakeNextFrameLocation DeltaSeconds) false true))))

(fn ConstructionScript)