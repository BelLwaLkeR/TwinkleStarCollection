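; Score manager actor for the MazePlanet main game scene that tracks the player's score and combo count.
; AddScore adds points from ComboScoreTable indexed by the current combo, capped at the last entry, then increments the combo.
; Score changes, including the reset on BeginPlay, are pushed to the HMD pawn's score text.
; ResetCombo clears the combo separately from the score, while AddCombo and SetResoultMode are empty stubs.
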(event Custom|SetResoultMode)

(event EventBeginPlay
  (CallFunction|ResetScore))

(event Collision|EventActorBeginOverlap
  (params (OtherActor :type Actor%20Object%20Reference)))

(event EventTick
  (params (DeltaSeconds :type Float%20%28single-precision%29)))

(fn ConstructionScript)

(fn AddScore
  (bind _comboscoretable (Variables|Default|GetComboScoreTable))
  (bind _returnvalue (Utilities|Array|LastIndex _comboscoretable))
  (bind _output_get (Variables|Default|SetScore (+ (Variables|Default|GetScore) (Utilities|Array|Get(acopy) (Variables|Default|GetComboScoreTable) (select (> _returnvalue (Variables|Default|GetCombo)) (Variables|Default|GetCombo) _returnvalue)))))
  (bind _output_get_2 (Variables|Default|SetCombo (+ (Variables|Default|GetCombo) 1)))
  (CallFunction|UpdateScoreUI)
  (return (Utilities|Array|Get(acopy) (Variables|Default|GetComboScoreTable) (select (> _returnvalue (Variables|Default|GetCombo)) (Variables|Default|GetCombo) _returnvalue)) _output_get _output_get_2))

(fn GetScore
  (return (Variables|Default|GetScore)))

(fn ResetScore
  (Variables|Default|SetScore 0)
  (CallFunction|UpdateScoreUI))

(fn UpdateScoreUI
  (Default|SetScoreText (Variables|Default|GetHMDPawn) (Variables|Default|GetScore)))

(fn AddCombo)

(fn ResetCombo
  (Variables|Default|SetCombo 0))