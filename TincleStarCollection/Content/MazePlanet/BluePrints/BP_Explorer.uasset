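; BP_Explorer is an actor that walks across a spherical planet toward the HMD's teleport pin while the player looks at the planet.
; Each tick, RotateToPlanet aligns its capsule's up axis away from the planet center and its forward axis toward the pin using MakeRotFromZX.
; Landing then snaps it to the planet radius, and MoveForward steps it by Speed until it nears the pin.
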(event OnComponentHit(CapsuleComponent)
  (params (HitComponent :type Primitive%20Component%20Object%20Reference) (OtherActor :type Actor%20Object%20Reference) (OtherComp :type Primitive%20Component%20Object%20Reference) (NormalImpulse :type Vector :default "0, 0, 0") (Hit :type Hit%20Result%20Structure%20%28by%20ref%29))
  (if (and (not (Variables|Default|GetIsLanded)) (== OtherActor 0))
    (Variables|Default|SetIsLanded true)))

(event EventBeginPlay
  (CallFunction|RotatetoPlanet true))

(event EventTick
  (params (DeltaSeconds :type Float%20%28single-precision%29))
  (bind _islooking (Default|IsLookingPlanet (Variables|Default|GetHMDLocation)))
  (if _islooking
    (CallFunction|RotatetoPlanet false)
    (CallFunction|Landing)
    (CallFunction|MoveForward (Variables|Default|GetDontMoveDistance))))

(fn ConstructionScript)

(fn RotatetoPlanet
  (params (Initialize :type Boolean))
  (LocalVariables|SetInitializeFlag Initialize)
  (Utilities|FlowControl|Sequence
    (:then_0
      (|SetExplorerPosition))
    (:then_1
      (|SetPlanetPosition))
    (:then_2
      (bind _returnvalue (|SetExplorerToPlanetDistance)))
    (:then_3
      (|RotateExplorer))
    (:then_4
      (return))))

(fn MoveForward
  (params (DontMoveDistance :type Float%20%28single-precision%29))
  (bind _islooking (Default|IsLookingPlanet (Variables|Default|GetHMDLocation)))
  (if _islooking
    (if (< (* (Variables|Default|GetSpeed) DontMoveDistance) (Math|Vector|VectorLength (- (Transformation|GetWorldLocation (Variables|/Game/MazePlanet/BluePrints/HMDLocomotionPawn.HMDLocomotionPawn_C|GetTeleportPin (Variables|Default|GetHMDLocation))) (Transformation|GetWorldLocation (Variables|Collision|GetCapsuleComponent)))))
      (Transformation|SetActorLocation (+ (* (Math|Vector|RotateVector (Math|Vector|MakeVector 1.0 0.0 0.0) (Transformation|GetWorldRotation (Variables|Collision|GetCapsuleComponent))) (Variables|Default|GetSpeed)) (Transformation|GetWorldLocation (Variables|Collision|GetCapsuleComponent))) false true))))

(fn Landing
  (bind _capsulecomponent (Variables|Collision|GetCapsuleComponent))
  (bind _returnvalue (Transformation|GetWorldLocation _capsulecomponent))
  (Transformation|SetWorldLocation (Variables|Collision|GetCapsuleComponent) (+ (* (* (Math|Vector|GetUpVector (Variables|Collision|GetCapsuleComponent)) -1) (- (Math|Vector|VectorLength (- (Transformation|GetWorldLocation (Variables|/Game/MazePlanet/BluePrints/Planet.Planet_C|GetSphere (Variables|Default|GetPlanet))) _returnvalue)) (Variables|Default|GetPlanetRadius))) _returnvalue) false true))

(fn RotationtoTarget
  (bind _capsulecomponent (Variables|Collision|GetCapsuleComponent))
  (bind _hmdlocation (Variables|Default|GetHMDLocation))
  (bind _returnvalue (Transformation|GetWorldLocation _capsulecomponent))
  (bind _teleportpin (Variables|/Game/MazePlanet/BluePrints/HMDLocomotionPawn.HMDLocomotionPawn_C|GetTeleportPin _hmdlocation))
  (bind _returnvalue_2 (Transformation|GetWorldLocation _teleportpin))
  (bind _returnvalue_3 (- _returnvalue _returnvalue_2))
  (bind (_x _y) (Math|Vector|BreakVector _returnvalue_3))
  (Transformation|SetWorldRotation (Variables|Collision|GetCapsuleComponent) (Math|Rotator|FindLookatRotation _returnvalue (+ _returnvalue (Math|Vector|RotateVector (Math|Vector|MakeVector _x _y 0.0) (Transformation|GetWorldRotation (Variables|Collision|GetCapsuleComponent))))) false false))