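; Planet actor for MazePlanet that adjusts its vertical position relative to the VR player's view.
; On BeginPlay it teleports to the height of the HMD's VR origin and stores that spot as its default position.
; SetHeightFromSight projects the given eye pitch across the horizontal camera-to-planet distance using tangent, then teleports the planet to that height, clamped between lowest and highest limits.
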(event EventBeginPlay
  (bind _returnvalue (Transformation|GetActorLocation))
  (bind _hmdlocation (Variables|Default|GetHMDLocation))
  (bind (_x _y) (Math|Vector|BreakVector _returnvalue))
  (bind _vrorigin (Variables|/Game/MazePlanet/BluePrints/Player.Player_C|GetVROrigin _hmdlocation))
  (bind _returnvalue_2 (Transformation|GetWorldLocation _vrorigin))
  (bind _z (Math|Vector|BreakVector _returnvalue_2))
  (bind _returnvalue_3 (Math|Vector|MakeVector _x _y _z))
  (Transformation|SetActorLocation _returnvalue_3 false true)
  (Variables|Default|SetdefaultPosition _returnvalue_3))

(event EventTick
  (params (DeltaSeconds :type Float%20%28single-precision%29)))

(fn ConstructionScript)

(fn SetHeightfromSight
  (params (cameraLoction :type Vector) (eyeAngle :type Rotator))
  (bind (_x _y) (Math|Vector|BreakVector cameraLoction))
  (bind _returnvalue (Transformation|GetActorLocation))
  (bind _returnvalue_2 (Transformation|GetActorLocation))
  (bind (_x_2 _y_2) (Math|Vector|BreakVector _returnvalue))
  (bind (_x_3 _y_3) (Math|Vector|BreakVector _returnvalue_2))
  (Transformation|SetActorLocation (Math|Vector|MakeVector _x_2 _y_2 (Math|Float|Clamp(Float) (+ (* (Math|Trig|Tan(Degrees) (.Pitch (Math|Rotator|BreakRotator eyeAngle))) (Math|Vector2D|Vector2DLength (- (Math|Vector2D|MakeVector2D _x _y) (Math|Vector2D|MakeVector2D _x_3 _y_3)))) (.Z (Math|Vector|BreakVector cameraLoction))) (Variables|Default|GetlowestHeight) (Variables|Default|GethighestHeight))) false true))