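; Title-scene star that acts as the game's start trigger, loading the GameMain level when the explorer actor hits it.
; On BeginPlay it moves out along its direction from the planet by a spawn distance, then falls toward the planet each Tick with a swept, spinning motion.
; A planet hit switches it to landed, where it spins around the planet-facing axis and shows a text label oriented away from the planet.
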(event OnComponentHit(Sphere)
  (params (HitComponent :type Primitive%20Component%20Object%20Reference) (OtherActor :type Actor%20Object%20Reference) (OtherComp :type Primitive%20Component%20Object%20Reference) (NormalImpulse :type Vector :default "0, 0, 0") (Hit :type Hit%20Result%20Structure%20%28by%20ref%29)))

(event OnComponentHit(StaticMesh)
  (params (HitComponent :type Primitive%20Component%20Object%20Reference) (OtherActor :type Actor%20Object%20Reference) (OtherComp :type Primitive%20Component%20Object%20Reference) (NormalImpulse :type Vector :default "0, 0, 0") (Hit :type Hit%20Result%20Structure%20%28by%20ref%29))
  (if (== OtherActor (Variables|Default|GetExplorerActor))
    (CallFunction|Burst)
    (elif (and (== OtherActor (Variables|Default|GetPlanetActor)) (not (Variables|Default|GetisLanding)))
      (Variables|Default|SetisLanding true))))

(event Custom|burst
  (Game|OpenLevel(byName) "GameMain"))

(event EventBeginPlay
  (|SetupLocation))

(event EventTick
  (params (DeltaSeconds :type Float%20%28single-precision%29))
  (if (Variables|Default|GetisLanding)
    (CallFunction|Landing 0.5)
    (else
      (CallFunction|Falling 6.0))))

(fn ConstructionScript)

(fn Landing
  (params (RotationSpeed :type Float%20%28single-precision%29))
  (bind _staticmesh (Variables|Default|GetStaticMesh))
  (bind _returnvalue (Transformation|GetWorldLocation _staticmesh))
  (Transformation|AddLocalRotation (Variables|Default|GetStaticMesh) (Math|Vector|RotatorfromAxisandAngle (Math|Vector|Normalize (- (Transformation|GetWorldLocation (Variables|/Game/MazePlanet/BluePrints/Planet.Planet_C|GetSphere (Variables|Default|GetPlanetActor))) (Transformation|GetWorldLocation (Variables|Default|GetStaticMesh)))) RotationSpeed) false false)
  (Rendering|SetVisibility (Variables|Default|GetTextRender) true false)
  (Transformation|SetWorldLocationAndRotation (Variables|Default|GetTextRender) (+ _returnvalue (* (Transformation|GetActorScale3D) "0, 0,-2.000000")) (Math|Rotator|FindLookatRotation (Transformation|GetWorldLocation (Variables|/Game/MazePlanet/BluePrints/Planet.Planet_C|GetSphere (Variables|Default|GetPlanetActor))) _returnvalue) false true))

(fn Falling
  (params (RollingSpeedDegree :type Float%20%28single-precision%29))
  (Transformation|AddLocalRotation (Variables|Default|GetStaticMesh) (Math|Rotator|MakeRotator 0.0 0.0 RollingSpeedDegree) false false)
  (Transformation|AddWorldOffset (Variables|Default|GetStaticMesh) (* (Math|Vector|Normalize (- (Transformation|GetWorldLocation (Variables|/Game/MazePlanet/BluePrints/Planet.Planet_C|GetSphere (Variables|Default|GetPlanetActor))) (Transformation|GetWorldLocation (Variables|Default|GetStaticMesh)))) (Variables|Default|GetFallSpeed)) true false))