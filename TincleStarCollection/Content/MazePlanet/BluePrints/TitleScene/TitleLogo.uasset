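; Title-scene logo actor that repositions itself every tick and turns to face the player camera.
; BeginPlay stores its horizontal distance from the planet.
; MakeNewPosition holds math that scales the camera-to-planet 2D direction by that distance and keeps the actor's height, without adding the planet's location.
; Tick teleports the actor to MakeNewPosition's result with a look-at rotation toward the camera.
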(event EventBeginPlay
  (|SetDefaultDistanceFromPanet))

(event Collision|EventActorBeginOverlap
  (params (OtherActor :type Actor%20Object%20Reference)))

(event EventTick
  (params (DeltaSeconds :type Float%20%28single-precision%29))
  (bind _returnvalue (|MakeNewPosition))
  (Transformation|SetActorLocationAndRotation _returnvalue (Math|Rotator|FindLookatRotation _returnvalue (Transformation|GetWorldLocation (Variables|/Game/MazePlanet/BluePrints/Player.Player_C|GetCamera (Variables|Default|Getplayer)))) false true))

(fn ConstructionScript)