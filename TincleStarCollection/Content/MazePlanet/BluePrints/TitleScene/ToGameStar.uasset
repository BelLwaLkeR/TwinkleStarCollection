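; Title-scene star pickup on the planet that starts the game when the explorer reaches it.
; After a one-second delay it is placed on the planet's far side from the player camera and activated.
; Each tick it follows the planet's height offset, spins about the planet's radial axis and tests squared distance to the explorer.
; Collection plays a sound, clears the player's curtain-open flag, then loads GameMain after a delay.
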(event Custom|ResetPosition
  (|SetDefaultLocation))

(event Custom|GetStar
  (Audio|PlaySound2D "/Game/MazePlanet/Sounds/get2.get2" 1.0 1.0)
  (Variables|/Game/MazePlanet/BluePrints/Player.Player_C|SettoOpenCurtain (Variables|Default|Getplayer) false)
  (Utilities|FlowControl|Delay 1.0)
  (Game|OpenLevel(byName) "GameMain"))

(event EventBeginPlay
  (Variables|Default|SetisActive false)
  (Utilities|FlowControl|Delay 1.0)
  (CallFunction|ResetPosition)
  (Variables|Default|SetisActive true))

(event EventTick
  (params (DeltaSeconds :type Float%20%28single-precision%29))
  (|SetHeightOffsetFromPlanet)
  (|CheckHitExplorer
    (:else
      (CallFunction|Landing 0.5))))

(fn ConstructionScript)

(fn Landing
  (params (RotationSpeed :type Float%20%28single-precision%29))
  (Transformation|AddLocalRotation (Variables|Default|GetStaticMesh) (Math|Vector|RotatorfromAxisandAngle (Math|Vector|Normalize (- (Transformation|GetActorLocation (Variables|Default|GetPlanetActor)) (Transformation|GetActorLocation))) RotationSpeed) false false))

(fn Falling
  (params (RollingSpeedDegree :type Float%20%28single-precision%29) (FallSpeed :type Float%20%28single-precision%29))
  (bind _planetactor (Variables|Default|GetPlanetActor))
  (bind _collisionradius (Variables|/Game/MazePlanet/BluePrints/Planet.Planet_C|GetCollisionRadius _planetactor))
  (Transformation|AddLocalRotation (Variables|Default|GetStaticMesh) (Math|Rotator|MakeRotator 0.0 0.0 RollingSpeedDegree) false false)
  (Transformation|AddActorWorldOffset (* (Math|Vector|Normalize (- (Transformation|GetActorLocation (Variables|Default|GetPlanetActor)) (Transformation|GetActorLocation))) FallSpeed) false true)
  (if (<= (Math|Vector|VectorLengthSquared (- (Transformation|GetActorLocation) (Transformation|GetActorLocation (Variables|Default|GetPlanetActor)))) (Variables|/Game/MazePlanet/BluePrints/Planet.Planet_C|GetCollisionRadius (Variables|Default|GetPlanetActor)))
    (Transformation|SetActorLocation (+ (* (Math|Vector|Normalize (- (Transformation|GetActorLocation (Variables|Default|GetPlanetActor)) (Transformation|GetActorLocation))) _collisionradius) (Transformation|GetActorLocation (Variables|Default|GetPlanetActor))) false true)
    (else
      (Development|PrintString (Utilities|String|ToString(Float) _collisionradius)))))

(fn RandomFloat
  (params (min :type Float%20%28single-precision%29) (max :type Float%20%28single-precision%29))
  (return (+ min (* (Math|Random|RandomFloat) (- max min)))))

(fn GetIsActive
  (return (Variables|Default|GetisActive)))