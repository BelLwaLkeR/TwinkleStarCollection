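; WalkSignBoard is a title-scene signboard actor with left and right text renders that appear when ToGameStar is active.
; Both texts are hidden on BeginPlay.
; While ToGameStar is active, Tick shows them and rebuilds the board's rotation every frame.
; MakeRotFromYZ pins the board's Y axis to world up and aims its Z axis along the direction from ToGameStar toward Planet.
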(event EventBeginPlay
  (Rendering|SetVisibility (Variables|Default|GetTextRenderR) false false))

(event Collision|EventActorBeginOverlap
  (params (OtherActor :type Actor%20Object%20Reference)))

(event EventTick
  (params (DeltaSeconds :type Float%20%28single-precision%29))
  (if (Variables|/Game/MazePlanet/BluePrints/TitleScene/ToGameStar.ToGameStar_C|GetisActive (Variables|Default|GettoGameStar))
    (Transformation|SetActorRotation (Class|KismetMathLibrary|MakeRotfromYZ (Math|Vector|MakeVector 0.0 0.0 1.0) (- (Transformation|GetActorLocation (Variables|Default|Getplanet)) (Transformation|GetActorLocation (Variables|Default|GettoGameStar)))) true)
    (Rendering|SetVisibility (Variables|Default|GetTextRenderR) true false)))

(fn ConstructionScript)